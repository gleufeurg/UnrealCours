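; BPC_Command is a Blueprint component for a Command pattern setup, holding an array of commands and a current index.
; On BeginPlay it constructs a Move_Command with its owner as the Unit and appends it to the array.
; Debug keys P and O step the index forward and back within bounds with colored prints, while Space prints it.
; No command is executed or undone here.
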(event EventBeginPlay
  (bind _returnvalue (Game|ConstructObjectfromClass "/Game/CommandPattern/Move_Command.Move_Command_C" (Components|GetOwner)))
  (Utilities|Array|Add (Variables|Default|Getcommand) _returnvalue))

(event Input|KeyboardEvents|DebugKeyO
  (params (Key :type Key%20Structure :default "None") (ActionValue :type Input%20Action%20Value%20Structure))
  (:Pressed
    (if (> (Variables|Default|GetcurrentIndex) 0)
      (bind _output_get (Variables|Default|SetcurrentIndex (- (Variables|Default|GetcurrentIndex) 1)))
      (Development|PrintString (Utilities|String|ToString(Integer) _output_get) true true "(R=1.000000,G=0.148505,B=0.258257,A=1.000000)" 1.0))))

(event Input|KeyboardEvents|DebugKeyP
  (params (Key :type Key%20Structure :default "None") (ActionValue :type Input%20Action%20Value%20Structure))
  (:Pressed
    (if (< (Variables|Default|GetcurrentIndex) (- (Utilities|Array|Length (Variables|Default|Getcommand)) 1))
      (bind _output_get (Variables|Default|SetcurrentIndex (+ (Variables|Default|GetcurrentIndex) 1)))
      (Development|PrintString (Utilities|String|ToString(Integer) _output_get) true true "(R=0.079966,G=1.000000,B=0.089627,A=1.000000)" 1.0))))

(event Input|KeyboardEvents|DebugKeySpaceBar
  (params (Key :type Key%20Structure :default "None") (ActionValue :type Input%20Action%20Value%20Structure))
  (:Pressed
    (Development|PrintString (Utilities|String|ToString(Integer) (Variables|Default|GetcurrentIndex)) true true "(R=0.045922,G=0.829911,B=1.000000,A=1.000000)" 1.0)))